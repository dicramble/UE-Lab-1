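; Second ball actor ("Sharik") that moves on its own and bounces off whatever blocks it, slowing with each hit.
; Tick moves it along Direction at Speed with a swept world offset, with no physics simulation in the graph.
; On a blocking hit, it reflects Direction about the surface normal, flattens Z to stay horizontal, and subtracts a tenth of its starting Speed, clamped at MinSpeed.
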(event `self.ReceiveBeginPlay`
  (set `self.Decelaration` (* (`self.Speed`) 0.1)))

(event `self.ReceiveTick`
  (params (DeltaSeconds :type "Float (single-precision)"))
  (bind _sweephitresult (`self.K2_AddActorWorldOffset` (* (* (`self.Direction`) (`self.Speed`)) DeltaSeconds) true))
  (bind (_bblockinghit _binitialoverlap _time _distance _location _impactpoint _normal) (`GameplayStatics.BreakHitResult` _sweephitresult))
  (if _bblockinghit
    (bind (_returnvalue_x _returnvalue_y) (`KismetMathLibrary.BreakVector` (`KismetMathLibrary.GetReflectionVector` (`self.Direction`) _normal)))
    (set `self.Direction` (`KismetMathLibrary.MakeVector` _returnvalue_x _returnvalue_y))
    (set `self.Speed` (`KismetMathLibrary.FMax` (- (`self.Speed`) (`self.Decelaration`)) (`self.MinSpeed`)))))

(fn `UserConstructionScript`)
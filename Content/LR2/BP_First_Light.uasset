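; BP_First_Light is a blinking point light that adds a disco effect by changing color at random.
; On BeginPlay, a DoN node loops back through a Delay of Duration, toggling the PointLight's visibility on each pass until it has run 2×Count−1 times.
; Each pass also assigns random RGB values to the light color before the toggle.
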(event `self.ReceiveBeginPlay`
  (`/Engine/EditorBlueprintResources/StandardMacros.Do N` (+ (`self.Count`) (- (`self.Count`) 1)) :!label _label
    (:`Exit`
      (`KismetSystemLibrary.Delay` (`self.Duration`))
      (bind _structout (setmembers `LinearColor` :`StructRef` (`LightComponentBase.GetLightColor` (`self.PointLight`)) :`R` (`KismetMathLibrary.RandomFloatInRange` 0.0 1.0) :`G` (`KismetMathLibrary.RandomFloatInRange` 0.0 1.0) :`B` (`KismetMathLibrary.RandomFloatInRange` 0.0 1.0) :`A` 1.0)) ; Я еще вне задания решила небольшую дискотеку устроить)
      (`LightComponent.SetLightColor` (`self.PointLight`) _structout false)
      (`SceneComponent.ToggleVisibility` (`self.PointLight`) false)
      (goto _label))))

(fn `UserConstructionScript`)